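; Player controller Blueprint that puts the main HUD on screen when it possesses a pawn.
; On Possess, it calls the parent handler, then creates a MainHUD widget owned by itself and adds it to the viewport, only if it is a local controller.
; Debug prints show the controller's name and the result of the local check.
; BeginPlay, Tick and the construction script are empty.
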(event `self.ReceiveBeginPlay`)

(event `self.ReceivePossess`
  (params (PossessedPawn :type "Pawn Object Reference"))
  (`parent.ReceivePossess` PossessedPawn)
  (`KismetSystemLibrary.PrintString` (`KismetSystemLibrary.GetDisplayName` self) true true (struct :`G` 0.66 :`B` 1.0 :`A` 1.0) 10.0)
  (if (`self.IsLocalController`)
    (`KismetSystemLibrary.PrintString` "Y" true true (struct :`G` 0.66 :`B` 1.0 :`A` 1.0) 10.0)
    (bind _returnvalue (`|CreateWidget` "/Game/UI/MainHUD.MainHUD_C" self))
    (`UserWidget.AddToViewport` _returnvalue 0)
    (else
      (`KismetSystemLibrary.PrintString` "N" true true (struct :`G` 0.66 :`B` 1.0 :`A` 1.0) 10.0))))

(fn `UserConstructionScript`)