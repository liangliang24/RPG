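; Player character Blueprint for Gideon, which sets up its UI and loads saved state when play begins.
; BeginPlay calls SpawnUI and then LoadFromState, neither of which is defined in this graph.
; A debug L key casts the game mode to RPGGameModeBaseBP to write the save game and prints a test string.
; Unwired leftover nodes hold earlier experiments with HUD creation, a delayed stun effect and a minion health widget.
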(event `self.ReceiveBeginPlay`
  (`self.SpawnUI`)
  (`self.LoadFromState`))

(event `self.ReceiveTick`
  (params (DeltaSeconds :type "Float (single-precision)")))

(event `Key|L`
  (params (Key :type "Key Structure"))
  (:`Pressed`
    (bind _asrpggame_mode_base_bp (cast `/Game/RPGGameModeBaseBP` (`GameplayStatics.GetGameMode`)))
    (`RPGGameModeBase.WriteSaveGame` _asrpggame_mode_base_bp)
    (`KismetSystemLibrary.PrintString` "Hello")))

(fn `UserConstructionScript`)