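; Cannon actor that automatically fires magic projectiles at the player.
; On BeginPlay it starts a looping half-second timer.
; Each tick of that timer spawns a MagicProjectileBP at the cannon's location, oriented toward player 0's character, then snaps the cannon's rotation to face the player.
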(event `self.ReceiveBeginPlay`
  (`KismetSystemLibrary.K2_SetTimerDelegate` (delegate `CustomEvent_0`) 0.5 true))

(event `CustomEvent_0`
  (bind _returnvalue (`KismetMathLibrary.Conv_VectorToRotator` (- (`self.K2_GetActorLocation` (`GameplayStatics.GetPlayerCharacter` 0)) (`self.K2_GetActorLocation`))))
  (`|SpawnActorFromClass` "/Game/MagicProjectileBP.MagicProjectileBP_C" (`KismetMathLibrary.MakeTransform` (`self.K2_GetActorLocation`) _returnvalue) "Undefined" "OverrideRootScale" null null)
  (`self.K2_SetActorRotation` _returnvalue true))

(fn `UserConstructionScript`)