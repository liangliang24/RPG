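; Aurora's E ability action, which spawns a ring of Ice actors when the action stops.
; StopAction runs the parent logic, then IceSpawn loops over indices 0 to 20, rotating a forward vector in 18-degree yaw steps to place each actor at a fixed radius around SpawnCenter.
; Each actor's rotation derives from its outward offset, and spawning ignores collisions.
; SpawnCenter is read here but never set.
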(event `self.StopAction`
  (params (instigator :type "Actor Object Reference"))
  (`parent.StopAction` instigator)
  (`self.IceSpawn`))

(fn `IceSpawn`
  (bind _spawncenter (`self.SpawnCenter`))
  (for _index (range 21)
    (bind _returnvalue (+ _spawncenter (* (`KismetMathLibrary.Normal` (`KismetMathLibrary.GreaterGreater_VectorRotator` (`KismetMathLibrary.MakeVector` 1.0) (`KismetMathLibrary.MakeRotator` 0.0 0.0 (`KismetMathLibrary.Conv_IntToDouble` (* _index 18))))) 300.0)))
    (`|SpawnActorFromClass` "/Game/Character/Aurora/Ice.Ice_C" (`KismetMathLibrary.MakeTransform` _returnvalue (`KismetMathLibrary.Quat_Rotator` (`KismetMathLibrary.Conv_VectorToQuaternion` (- _returnvalue _spawncenter)))) "AlwaysSpawn" "OverrideRootScale" null null)))